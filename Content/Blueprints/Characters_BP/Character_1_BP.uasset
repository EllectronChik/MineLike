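; Player character for a voxel block-building game, with standard move, look and jump input and an on-screen debug readout of its position in block units.
; Attack and Cast share a camera line trace, nudged along the hit normal, to call ModifyVoxel on the hit ChunkBase, removing or placing a block.
; Placement is skipped when the new block would overlap the player's capsule.
; Five inventory slot inputs select the block type to place.
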(event EventBeginPlay)

(event Collision|EventActorBeginOverlap
  (params (OtherActor :type Actor%20Object%20Reference)))

(event EventTick
  (params (DeltaSeconds :type Float%20%28single-precision%29))
  (Development|PrintString (Utilities|String|ToString(Vector) (/ (Transformation|GetActorLocation) (Variables|Default|GetBlockSize))) true true "(R=0.000000,G=0.660000,B=1.000000,A=1.000000)" DeltaSeconds "."))

(event Input|ActionEvents|InputActionJump
  (params (Key :type Key%20Structure :default "None"))
  ;[1 1 1] Controlling
  (:Pressed
    (Character|Jump))
  (:Released
    (Character|StopJumping)))

(event Input|ActionEvents|InputActionAttack
  (params (Key :type Key%20Structure :default "None"))
  ;[1 1 1] Destoy Blocks
  (:Pressed
    (bind (_returnvalue _outhit) (CallFunction|RayCast))
    (if _returnvalue
      (bind _aschunk_base (Utilities|Casting|CastToChunkBase (.HitActor (Collision|BreakHitResult _outhit))))
      (Class|ChunkBase|ModifyVoxel _aschunk_base (Class|VoxelFunctionLibrary|WorldtoLocalBlockPosition (- (.Location (Collision|BreakHitResult _outhit)) (.Normal (Collision|BreakHitResult _outhit))) (Variables|Default|GetChunkSize)) "Air"))))

(event Input|ActionEvents|InputActionCast
  (params (Key :type Key%20Structure :default "None"))
  ;[1 1 1] Block Placement
  (:Pressed
    (bind (_returnvalue _outhit) (CallFunction|RayCast))
    (if _returnvalue
      (if (not (Class|VoxelFunctionLibrary|IsObjectCollidewithPlayer (Variables|Collision|GetCapsuleComponent) (Math|Conversions|ToVector(Float) (Class|VoxelFunctionLibrary|GetBlockCenterPosition (- (.Location (Collision|BreakHitResult _outhit)) (.Normal (Collision|BreakHitResult _outhit))) (.Normal (Collision|BreakHitResult _outhit)) (Variables|Default|GetBlockSize))) (Variables|Default|GetBlockSize)))
        (bind _aschunk_base (Utilities|Casting|CastToChunkBase (.HitActor (Collision|BreakHitResult _outhit))))
        (Class|ChunkBase|ModifyVoxel _aschunk_base (Class|KismetMathLibrary|FTruncVector (+ (.Normal (Collision|BreakHitResult _outhit)) (Class|VoxelFunctionLibrary|WorldtoLocalBlockPosition (- (.Location (Collision|BreakHitResult _outhit)) (.Normal (Collision|BreakHitResult _outhit))) (Variables|Default|GetChunkSize)))) (Variables|Default|GetBlock))))))

(event Input|ActionEvents|InputActionFirstInventorySlot
  (params (Key :type Key%20Structure :default "None"))
  ;[1 1 1] SetBlock
  (:Pressed
    (Variables|Default|SetBlock "Planks")))

(event Input|ActionEvents|InputActionSecondInventorySlot
  (params (Key :type Key%20Structure :default "None"))
  ;[1 1 1] SetBlock
  (:Pressed
    (Variables|Default|SetBlock "Stone")))

(event Input|ActionEvents|InputActionThirdInventorySlot
  (params (Key :type Key%20Structure :default "None"))
  ;[1 1 1] SetBlock
  (:Pressed
    (Variables|Default|SetBlock "Dirt")))

(event Input|ActionEvents|InputActionForthInventorySlot
  (params (Key :type Key%20Structure :default "None"))
  ;[1 1 1] SetBlock
  (:Pressed
    (Variables|Default|SetBlock "Grass")))

(event Input|ActionEvents|InputActionFifthInventorySlot
  (params (Key :type Key%20Structure :default "None"))
  ;[1 1 1] SetBlock
  (:Pressed
    (Variables|Default|SetBlock "Glass")))

(event Input|AxisEvents|InputAxisLook_Up
  (params (AxisValue :type Float%20%28single-precision%29))
  ;[1 1 1] Controlling
  (Pawn|Input|AddControllerPitchInput AxisValue))

(event Input|AxisEvents|InputAxisTurn
  (params (AxisValue :type Float%20%28single-precision%29))
  ;[1 1 1] Controlling
  (Pawn|Input|AddControllerYawInput AxisValue))

(event Input|AxisEvents|InputAxisMoveForward
  (params (AxisValue :type Float%20%28single-precision%29))
  ;[1 1 1] Controlling
  (Pawn|Input|AddMovementInput (Math|Vector|GetForwardVector (Math|Rotator|MakeRotator 0.0 0.0 (.yaw (Pawn|GetControlRotation :!class /Script/Engine.Pawn)))) AxisValue false))

(event Input|AxisEvents|InputAxisMoveRight
  (params (AxisValue :type Float%20%28single-precision%29))
  ;[1 1 1] Controlling
  (Pawn|Input|AddMovementInput (Math|Vector|GetRightVector (Math|Rotator|MakeRotator 0.0 0.0 (.yaw (Pawn|GetControlRotation :!class /Script/Engine.Pawn)))) AxisValue false))

(fn ConstructionScript)

(fn RayCast
  (bind _returnvalue (Pawn|GetLocalViewingPlayerController))
  (bind _playercameramanager (Variables|/Script/Engine.PlayerController|GetPlayerCameraManager _returnvalue))
  (bind _returnvalue_2 (Camera|GetCameraLocation _playercameramanager))
  (bind (_outhit _returnvalue_3) (Collision|LineTraceByChannel _returnvalue_2 (+ _returnvalue_2 (* (Math|Vector|GetForwardVector (Camera|GetCameraRotation _playercameramanager)) (Variables|Default|GetBlockDistance))) "TraceTypeQuery1" false 0 "None" true "(R=1.000000,G=0.000000,B=0.000000,A=1.000000)" "(R=0.000000,G=1.000000,B=0.000000,A=1.000000)" 1e+01))
  (return _returnvalue_3 _outhit))